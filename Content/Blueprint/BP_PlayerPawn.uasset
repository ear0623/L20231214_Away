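; BP_PlayerPawn is the player-controlled propeller plane, which flies constantly forward and can fire missiles.
; Tick feeds the actor's forward vector into movement input, while Roll and Pitch axes add frame-time-scaled local rotation.
; BeginPlay registers the propeller mesh with BPRotateComponent.
; Fire spawns a BP_Missile at the actor transform with the pawn as owner and instigator, and Accelrate toggles IsBoost, which this graph never reads.
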(event `self.ReceiveBeginPlay`
  ;[0 0 0] BeginPlay
  (`KismetArrayLibrary.Array_Add` (`/Game/Blueprint/BP_RotateComponent.SceneComponent` (`self.BP_RotateComponent`)) (`self.SM_P38_Propeller`)))

(event `InputAxis|Roll`
  (params (AxisValue :type "Float (single-precision)"))
  ;[0 0 0] Movement
  (`self.K2_AddActorLocalRotation` (`KismetMathLibrary.MakeRotator` (* AxisValue (`GameplayStatics.GetWorldDeltaSeconds`) (`self.Rotate`)))))

(event `self.ReceiveTick`
  (params (DeltaSeconds :type "Float (single-precision)"))
  ;[0 0 0] Movement
  (`self.AddMovementInput` (`KismetMathLibrary.GetForwardVector` (`self.K2_GetActorRotation`))))

(event `InputAxis|Pitch`
  (params (AxisValue :type "Float (single-precision)"))
  ;[0 0 0] Movement
  (`self.K2_AddActorLocalRotation` (`KismetMathLibrary.MakeRotator` 0.0 (* AxisValue (`GameplayStatics.GetWorldDeltaSeconds`) (`self.Rotate`)))))

(event `InputAction|Fire`
  (params (Key :type "Key Structure"))
  ;[0 0 0] Fire
  (:`Pressed`
    (`|SpawnActorFromClass` "/Game/Blueprint/BP_Missile.BP_Missile_C" (`self.GetTransform` self) "Undefined" "MultiplyWithRoot" self self)))

(event `InputAction|Accelrate`
  (params (Key :type "Key Structure"))
  ;[0 0 0] Boost
  (:`Pressed`
    (set `self.bIsBoost` true))
  (:`Released`
    (set `self.bIsBoost` false)))

(fn `UserConstructionScript`)